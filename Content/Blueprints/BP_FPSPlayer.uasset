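; BP_FPSPlayer is the first-person shooter player that owns a weapon and fires it on player input.
; On BeginPlay it adds the default Enhanced Input mapping context for its player controller, then caches the ChildActor component's actor as its main BP_BaseWeapon.
; The IA_Fire Triggered event delegates shooting to that weapon's ShootWeapon function.
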(event `self.ReceiveBeginPlay`
  (bind `_as플레이어_컨트롤러` (cast `PlayerController` (`self.GetController`)))
  (bind _returnvalue (pcsubsystem `EnhancedInputLocalPlayerSubsystem` `_as플레이어_컨트롤러`))
  (`/Engine/EditorBlueprintResources/StandardMacros.IsValid` _returnvalue
    (:`Is Valid`
      (`EnhancedInputSubsystemInterface.AddMappingContext` _returnvalue "/Game/Input/IMC_DefaultContext.IMC_DefaultContext" 0 (struct))
      (bind _asbp_base_weapon (cast `/Game/Weapon/BP_BaseWeapon` (`ChildActorComponent.ChildActor` (`self.ChildActor`))))
      (set `self.MainWepaon` _asbp_base_weapon))))

(event `EnhancedInput|/Game/Input/Actions/IA_Fire`
  (params (ActionValue :type Boolean) (ElapsedSeconds :type "Float (double-precision)") (TriggeredSeconds :type "Float (double-precision)") (InputAction :type "InputAction Object Reference" :default "/Game/Input/Actions/IA_Fire.IA_Fire"))
  (:`Triggered`
    (`/Game/Weapon/BP_BaseWeapon.ShootWeapon` (`self.MainWepaon`))))

(fn `UserConstructionScript`)